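; Enemy melee attack gameplay ability that faces the combat target and plays a random tagged attack montage.
; When the montage's gameplay event fires, it searches a small sphere at the matching combat socket for live players.
; Non-friendly hits take damage and trigger blood effects, then one MeleeImpact gameplay cue plays, carrying the montage tag.
; The ability ends when the montage completes or is interrupted, or immediately if nothing is hit.
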(event `self.K2_ActivateAbility`
  (bind _returnvalue (`self.GetAvatarActorFromActorInfo`))
  (bind (_montage _montagetag _sockettag) (break `TaggedMontage` (`self.TargetMontage`)))
  (set `self.HasHitTarget` false)
  (`self.SettingTargetAndFacing`)
  (`self.SettingMontage`)
  (`AbilityTask_PlayMontageAndWait.CreatePlayMontageAndWaitProxy` "None" _montage 1.0 "None" false
    (:`then`
      (`AbilityTask_WaitGameplayEvent.WaitGameplayEvent` _montagetag null true
        (:`EventReceived`
          (bind _returnvalue_2 (message `CombatInterface.GetCombatSocketLocation` _returnvalue _sockettag))
          (bind _output_get (set `self.CombatSocketLocation` _returnvalue_2))
          (bind _outoverlappingactors (`AuraAbilitySystemLibrary.GetLivePlayerWithInRadius` _returnvalue (`|MakeArray` _returnvalue) 50.0 _output_get))
          (`self.ApplyDamage` _outoverlappingactors))))
    (:`OnCompleted`
      (`self.K2_EndAbility` :!label _label))
    (:`OnInterrupted`
      (goto _label))
    (:`OnCancelled`
      (goto _label))))

(fn `ApplyDamage`
  (params (Array :type "Array of Actor Object Reference"))
  (bind _returnvalue (`self.GetAvatarActorFromActorInfo`))
  (for _array_element Array
    (if (`AuraAbilitySystemLibrary.IsNotFriend` (`self.GetAvatarActorFromActorInfo`) _array_element)
      (`self.CauseDamage` _array_element)
      (set `self.HasHitTarget` true)
      (message `CombatInterface.GetBloodEffect` _array_element)))
  (if (`self.HasHitTarget`)
    (bind _returnvalue_2 (message `CombatInterface.GetCombatTarget` _returnvalue))
    (`self.K2_ExecuteGameplayCueWithParams` (struct :`TagName` "GameplayCue.MeleeImpact") (`AbilitySystemBlueprintLibrary.MakeGameplayCueParameters` 0.0 0.0 (struct) (struct) (struct) (`BlueprintGameplayTagLibrary.MakeGameplayTagContainerFromTag` (`.MontageTag` (break `TaggedMontage` (`self.TargetMontage`)))) (struct) (`self.CombatSocketLocation`) (0.0 0.0 0.0) null _returnvalue _returnvalue_2))
    (else
      (`self.K2_EndAbility`))))

(fn `SettingMontage`
  (bind _returnvalue (message `CombatInterface.GetAttackMontages` (`self.GetAvatarActorFromActorInfo`)))
  (set `self.TargetMontage` (`self.GetRandomTaggedMontage` _returnvalue))
  (return))

(fn `SettingTargetAndFacing`
  (bind _returnvalue (`self.GetAvatarActorFromActorInfo`))
  (bind _returnvalue_2 (message `CombatInterface.GetCombatTarget` _returnvalue))
  (bind _ascombat_interface (cast `CombatInterface` _returnvalue)
    (:`then`
      (`CombatInterface.UpdateFacingTarget` _ascombat_interface (`Actor.K2_GetActorLocation` _returnvalue_2)))
    (:`CastFailed`
      _))
  (return))
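; Enemy ranged attack Gameplay Ability that fires a projectile at the avatar's combat target.
; On activation it turns the avatar toward the target through CombatInterface and plays a random tagged montage from the avatar's attack montages.
; The montage's gameplay event tag times the shot, spawning the projectile from its socket toward the target's current location with optional pitch override.
; The ability then ends without stopping the montage.
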(event `self.K2_ActivateAbility`
  (bind (_montage _montagetag _sockettag) (break `TaggedMontage` (`self.TargetMontage`)))
  (`self.SettingTargetAndFacing`)
  (`self.SettingMontage`)
  (`AbilityTask_PlayMontageAndWait.CreatePlayMontageAndWaitProxy` "None" _montage 1.0 "None" false
    (:`then`
      (`AbilityTask_WaitGameplayEvent.WaitGameplayEvent` _montagetag null true
        (:`EventReceived`
          (bind _returnvalue (message `CombatInterface.GetCombatTarget` (`self.GetAvatarActorFromActorInfo`)))
          (`self.SpawnProjectile` (`Actor.K2_GetActorLocation` _returnvalue) _sockettag (`self.IsOverridePitch`) (`self.OverridePitch`))
          (`self.K2_EndAbility`))))))

(fn `SettingMontage`
  (bind _returnvalue (message `CombatInterface.GetAttackMontages` (`self.GetAvatarActorFromActorInfo`)))
  (set `self.TargetMontage` (`self.GetRandomTaggedMontage` _returnvalue))
  (return))

(fn `SettingTargetAndFacing`
  (bind _returnvalue (`self.GetAvatarActorFromActorInfo`))
  (bind _returnvalue_2 (message `CombatInterface.GetCombatTarget` _returnvalue))
  (bind _ascombat_interface (cast `CombatInterface` _returnvalue))
  (`CombatInterface.UpdateFacingTarget` _ascombat_interface (`Actor.K2_GetActorLocation` _returnvalue_2))
  (return))
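; Main menu scene actor that plays menu music, opens the WBP_MainMenu widget and spins a magic circle.
; BeginPlay adds the widget to the viewport, switches input to UI-only focused on it and shows the mouse cursor.
; Tick rolls MagicCircle at a frame-rate-independent rate.
; UpdateTime and SinTime provide a wrapping timer and scaled sine wave, but the graphs shown never call them.
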(event `self.ReceiveBeginPlay`
  (`GameplayStatics.PlaySound2D` "/Game/Assets/Sounds/Music/Music_MainMenu.Music_MainMenu" 1.0 1.0 0.0 null null)
  (bind _returnvalue (`|CreateWidget` "/Game/Assets/Sounds/UI/MainMenu/WBP_MainMenu.WBP_MainMenu_C"))
  (`UserWidget.AddToViewport` _returnvalue 0)
  (`WidgetBlueprintLibrary.SetInputMode_UIOnlyEx` (`GameplayStatics.GetPlayerController` 0) _returnvalue)
  (set `PlayerController.bShowMouseCursor` true (`GameplayStatics.GetPlayerController` 0)))

(event `self.ReceiveTick`
  (params (DeltaSeconds :type "Float (single-precision)"))
  (`SceneComponent.K2_AddLocalRotation` (`self.MagicCircle`) (`KismetMathLibrary.MakeRotator` (* (`GameplayStatics.GetWorldDeltaSeconds`) (`self.MagicCircleRotationRate`))) false false))

(fn `SinTime`
  (returns (ReturnValue :type "Float (double-precision)"))
  (return (* (`KismetMathLibrary.Sin` (`self.Time`)) (`self.Amplitude`))))

(fn `Update Time`
  (params (A :type "Float (double-precision)"))
  (bind _output_get (set `self.Time` (+ A (`self.Time`))))
  (if (> _output_get 6.3)
    (set `self.Time` 0.0)))

(fn `UserConstructionScript`)